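; PlateBP is a placeable plate that previews whether it can spawn, then becomes a physics object once activated.
; Before spawning, Plane overlaps toggle CanSpawn and swap between allow and disallow materials.
; ActiveObject enables physics and Box overlaps, applies the wall material and tags the root as a Plate; SkipBeginPlay bypasses preview setup, setting only collision type and tags.
; Overlaps with other plates, from Box or the spawned Plane, print a Game Over message.
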(event OnComponentBeginOverlap(Plane)
  (params (OverlappedComponent :type Primitive%20Component%20Object%20Reference) (OtherActor :type Actor%20Object%20Reference) (OtherComp :type Primitive%20Component%20Object%20Reference) (OtherBodyIndex :type Integer) (bFromSweep :type Boolean) (SweepResult :type Hit%20Result%20Structure%20%28by%20ref%29))
  (if (Variables|Default|Getis%20spawned)
    (if (Actor|ActorHasTag OtherActor "Plate")
      (Development|PrintString "Game Over (Plate Overlaps)"))
    (else
      (Variables|Default|Setcan%20spawn false)
      (Rendering|Material|SetMaterial (Variables|Default|GetPlane) 0 "/Game/Material/M_DisallowToSpawn.M_DisallowToSpawn"))))

(event OnComponentEndOverlap(Plane)
  (params (OverlappedComponent :type Primitive%20Component%20Object%20Reference) (OtherActor :type Actor%20Object%20Reference) (OtherComp :type Primitive%20Component%20Object%20Reference) (OtherBodyIndex :type Integer))
  (if (not (Variables|Default|Getis%20spawned))
    (Variables|Default|Setcan%20spawn true)
    (Rendering|Material|SetMaterial (Variables|Default|GetPlane) 0 "/Game/Material/M_AllowToSpawn.M_AllowToSpawn")))

(event OnComponentBeginOverlap(Box)
  (params (OverlappedComponent :type Primitive%20Component%20Object%20Reference) (OtherActor :type Actor%20Object%20Reference) (OtherComp :type Primitive%20Component%20Object%20Reference) (OtherBodyIndex :type Integer) (bFromSweep :type Boolean) (SweepResult :type Hit%20Result%20Structure%20%28by%20ref%29))
  (if (Components|ComponentHasTag (Variables|/Script/Engine.Actor|GetRootComponent OtherActor) "Plate")
    (Development|PrintString "Game Over (Plate Overlaps)")))

(event EventBeginPlay
  (if (Variables|Default|Getskip%20BeginPlay)
    (Collision|SetCollisionObjectType (Variables|Default|GetPlane) "ECC_WorldStatic")
    (Variables|/Script/Engine.ActorComponent|SetComponentTags (Variables|Default|GetDefaultSceneRoot) (Utilities|Array|MakeArray "Object" "Plate"))
    (else
      (Variables|Default|SetoriginMaterial%201 "/Game/StarterContent/Materials/M_Basic_Wall.M_Basic_Wall")
      (Rendering|Material|SetMaterial (Variables|Default|GetPlane) 0 "/Game/Material/M_AllowToSpawn.M_AllowToSpawn"))))

(event Collision|EventActorBeginOverlap
  (params (OtherActor :type Actor%20Object%20Reference)))

(event EventTick
  (params (DeltaSeconds :type Float%20%28single-precision%29)))

(fn ConstructionScript)

(fn ActiveObject
  (bind _plane (Variables|Default|GetPlane))
  (Collision|SetCollisionObjectType _plane "ECC_WorldStatic")
  (Physics|SetSimulatePhysics _plane true)
  (Variables|Default|Setis%20spawned true)
  (Rendering|Material|SetMaterial (Variables|Default|GetPlane) 0 (Variables|Default|GetoriginMaterial%201))
  (Variables|/Script/Engine.ActorComponent|SetComponentTags (Variables|Default|GetDefaultSceneRoot) (Utilities|Array|MakeArray "Object" "Plate"))
  (Variables|/Script/Engine.PrimitiveComponent|SetbGenerateOverlapEvents (Variables|Default|GetBox) true))