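; Player pawn for placing mugs and plates in the level, with an orbit, zoom and vertical-move camera.
; Creates the IngameSingleWB widget, whose selection events set the class to spawn.
; Left press spawns it and opens a Tick gate that snaps it to the cursor's surface hit, aligned to the normal.
; Release activates it if its CanSpawn flag is true, otherwise destroys it, casting by class display name.
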(event Custom|Select%20Object%20to%20MugCup
  (Variables|Default|Setselected%20object "/Game/Blueprint/MugCupBP.MugCupBP_C"))

(event Custom|Select%20Object%20to%20Plate
  (Variables|Default|Setselected%20object "/Game/Blueprint/PlateBP.PlateBP_C"))

(event EventBeginPlay
  (bind _returnvalue (Game|GetPlayerController 0))
  (bind _springarm (Variables|Default|GetSpringArm))
  ;[1 1 1] 초기화
  (Variables|Default|Setselected%20object 0)
  (Transformation|SetWorldLocationAndRotation _springarm "0, 0, 0" "0, 0, 0" false false)
  (Pawn|SetControlRotation (Game|GetPlayerController 0) (Math|Rotator|MakeRotator 0.0 -2e+01 2.3e+02))
  (Variables|/Script/Engine.SpringArmComponent|SetTargetArmLength _springarm 6e+02)
  (bind _returnvalue_2 (UserInterface|CreateWidget "/Game/UI/IngameSingleWB.IngameSingleWB_C"))
  (UserInterface|Viewport|AddtoViewport _returnvalue_2 0)
  (Input|SetInputModeGameandUI _returnvalue 0 "LockOnCapture" false)
  (Variables|/Script/Engine.PlayerController|SetbShowMouseCursor _returnvalue true)
  (EventDispatchers|BindEventtoMugCupSelect _returnvalue_2 (delegate Custom|Select%20Object%20to%20MugCup))
  (EventDispatchers|BindEventtoPlateSelect _returnvalue_2 (delegate Custom|Select%20Object%20to%20Plate)))

(event Collision|EventActorBeginOverlap
  (params (OtherActor :type Actor%20Object%20Reference)))

(event EventTick
  (params (DeltaSeconds :type Float%20%28single-precision%29))
  (bind _returnvalue (Game|GetPlayerController 0))
  (bind _array (Utilities|Array|MakeArray "ObjectTypeQuery1"))
  (bind _hitresult (Class|PlayerController|GetHitResultUnderCursorforObjects _returnvalue _array true))
  (bind (_bblockinghit _binitialoverlap _time _distance _location _impactpoint _normal) (Collision|BreakHitResult _hitresult))
  (Utilities|FlowControl|Sequence
    (:then_0
      ;[1 1 1] 오브젝트 생성
      (Utilities|FlowControl|Gate true
        (:Exit
          (Transformation|SetActorLocationAndRotation (Variables|Default|Gettarget) _location (Math|Rotator|MakeRotfromZ _normal)))))
    (:then_1
      ;[1 1 1] 카메라 움직임
      (Utilities|FlowControl|Sequence
        (:then_0
          (if (Variables|Default|GetCameraUp)
            (Pawn|Input|AddMovementInput "0, 0,1.000000" 1.0 false)))
        (:then_1
          (if (Variables|Default|GetCameraDown)
            (Pawn|Input|AddMovementInput "0, 0,1.000000" -1.0 false)))))))

(event Input|MouseEvents|MouseX
  (params (AxisValue :type Float%20%28single-precision%29))
  ;[1 1 1] 카메라 움직임
  (if (Variables|Default|GetCameraMovable)
    (Pawn|Input|AddControllerYawInput AxisValue)))

(event Input|MouseEvents|MouseY
  (params (AxisValue :type Float%20%28single-precision%29))
  ;[1 1 1] 카메라 움직임
  (if (Variables|Default|GetCameraMovable)
    (Pawn|Input|AddControllerPitchInput (* AxisValue -1.0))))

(event Input|MouseEvents|MouseWheelAxis
  (params (AxisValue :type Float%20%28single-precision%29))
  (bind _springarm (Variables|Default|GetSpringArm))
  ;[1 1 1] 카메라 움직임
  (Variables|/Script/Engine.SpringArmComponent|SetTargetArmLength _springarm (- (Variables|/Script/Engine.SpringArmComponent|GetTargetArmLength _springarm) (* AxisValue 2e+01))))

(event Input|MouseEvents|LeftMouseButton
  (params (Key :type Key%20Structure :default "None"))
  (bind _returnvalue (Game|GetPlayerController 0))
  (bind _array (Utilities|Array|MakeArray "ObjectTypeQuery1"))
  (bind _hitresult (Class|PlayerController|GetHitResultUnderCursorforObjects _returnvalue _array true))
  (bind (_bblockinghit _binitialoverlap _time _distance _location _impactpoint _normal) (Collision|BreakHitResult _hitresult))
  ;[1 1 1] 오브젝트 생성
  (:Pressed
    (if (Utilities|IsValidClass (Variables|Default|Getselected%20object))
      (CallFunction|CreateNewObject)
      (Utilities|FlowControl|Gate true) ; enters at Open
    ))
  (:Released
    (if (Utilities|IsValidClass (Variables|Default|Getselected%20object))
      (bind _can_spawn (CallFunction|CheckObjectCanSpawn))
      (if _can_spawn
        (Utilities|FlowControl|Sequence
          (:then_0
            (CallFunction|ActiveTargetObject)
            (Development|PrintString "turn over"))
          (:then_1
            (Utilities|FlowControl|Gate true) ; enters at Close
          ))
        (else
          (Utilities|FlowControl|Sequence
            (:then_0
              (Utilities|FlowControl|Gate true) ; enters at Close
            )
            (:then_1
              (Actor|DestroyActor (Variables|Default|Gettarget)))))))))

(event Input|MouseEvents|RightMouseButton
  (params (Key :type Key%20Structure :default "None"))
  ;[1 1 1] 카메라 움직임
  (:Pressed
    (Variables|Default|SetCameraMovable true))
  (:Released
    (Variables|Default|SetCameraMovable false)))

(event Input|KeyboardEvents|Q
  (params (Key :type Key%20Structure :default "None"))
  ;[1 1 1] 카메라 움직임
  (:Pressed
    (Variables|Default|SetCameraUp true))
  (:Released
    (Variables|Default|SetCameraUp false)))

(event Input|KeyboardEvents|E
  (params (Key :type Key%20Structure :default "None"))
  ;[1 1 1] 카메라 움직임
  (:Pressed
    (Variables|Default|SetCameraDown true))
  (:Released
    (Variables|Default|SetCameraDown false)))

(fn ConstructionScript)

(fn CreateNewObject
  (bind _returnvalue (Game|SpawnActorfromClass (Variables|Default|Getselected%20object) (Transformation|GetActorTransform) "Undefined" 0 0))
  (Variables|Default|Settarget _returnvalue))

(fn ActiveTargetObject
  (bind _target (Variables|Default|Gettarget))
  (switch string (Utilities|GetClassDisplayName (Variables|Default|Getselected%20object))
    (:MugCupBP_C
      (bind _asmug_cup_bp (Utilities|Casting|CastToMugCupBP _target))
      (Default|ActiveObject _asmug_cup_bp))
    (:PlateBP_C
      (bind _asplate_bp (Utilities|Casting|CastToPlateBP _target))
      (Default|ActiveObject _asplate_bp))))

(fn CheckObjectCanSpawn
  (bind _target (Variables|Default|Gettarget))
  (switch string (Utilities|GetClassDisplayName (Variables|Default|Getselected%20object))
    (:MugCupBP_C
      (bind _asmug_cup_bp (Utilities|Casting|CastToMugCupBP _target))
      (return (Variables|/Game/Blueprint/MugCupBP.MugCupBP_C|Getcan%20spawn _asmug_cup_bp)))
    (:PlateBP_C
      (bind _asplate_bp (Utilities|Casting|CastToPlateBP _target))
      (return (Variables|/Game/Blueprint/PlateBP.PlateBP_C|Getcan%20spawn _asplate_bp)))))