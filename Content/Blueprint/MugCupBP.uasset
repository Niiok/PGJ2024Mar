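; Placeable mug cup Blueprint that shows whether it can be spawned while in preview and takes on its real look once placed.
; Until spawned, root mesh overlaps clear CanSpawn and apply the disallow material to both slots; any end overlap re-allows it without checking remaining overlaps.
; SelectPreviewMesh and SetRealActor extend the parent's versions, applying allow/disallow preview materials or restoring the two original materials.
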(event OnComponentBeginOverlap(RootMesh)
  (params (OverlappedComponent :type Primitive%20Component%20Object%20Reference) (OtherActor :type Actor%20Object%20Reference) (OtherComp :type Primitive%20Component%20Object%20Reference) (OtherBodyIndex :type Integer) (bFromSweep :type Boolean) (SweepResult :type Hit%20Result%20Structure%20%28by%20ref%29))
  (bind _rootmesh (Variables|Default|GetRootMesh))
  (if (not (Variables|Default|GetbIsSpawned))
    (Variables|Default|SetbCanSpawn false)
    (Rendering|Material|SetMaterial _rootmesh 0 "/Game/Material/M_DisallowToSpawn.M_DisallowToSpawn")
    (Rendering|Material|SetMaterial _rootmesh 1 "/Game/Material/M_DisallowToSpawn.M_DisallowToSpawn")))

(event OnComponentEndOverlap(RootMesh)
  (params (OverlappedComponent :type Primitive%20Component%20Object%20Reference) (OtherActor :type Actor%20Object%20Reference) (OtherComp :type Primitive%20Component%20Object%20Reference) (OtherBodyIndex :type Integer))
  (bind _rootmesh (Variables|Default|GetRootMesh))
  (if (not (Variables|Default|GetbIsSpawned))
    (Variables|Default|SetbCanSpawn true)
    (Rendering|Material|SetMaterial _rootmesh 0 "/Game/Material/M_AllowToSpawn.M_AllowToSpawn")
    (Rendering|Material|SetMaterial _rootmesh 1 "/Game/Material/M_AllowToSpawn.M_AllowToSpawn")))

(event Collision|EventActorBeginOverlap
  (params (OtherActor :type Actor%20Object%20Reference)))

(event EventTick
  (params (DeltaSeconds :type Float%20%28single-precision%29)))

(fn ConstructionScript)

(fn SetRealActor
  (bind _rootmesh (Variables|Default|GetRootMesh))
  (|CallParentFunction)
  (Rendering|Material|SetMaterial _rootmesh 0 (Variables|Default|GetoriginMaterial%201))
  (Rendering|Material|SetMaterial _rootmesh 1 (Variables|Default|GetoriginMaterial%202)))

(fn SelectPreviewMesh
  (params (bPlacable :type Boolean))
  (bind _rootmesh (Variables|Default|GetRootMesh))
  (|CallParentFunction bPlacable)
  (if bPlacable
    (Rendering|Material|SetMaterial _rootmesh 0 "/Game/Material/M_AllowToSpawn.M_AllowToSpawn")
    (Rendering|Material|SetMaterial _rootmesh 1 "/Game/Material/M_AllowToSpawn.M_AllowToSpawn")
    (else
      (Rendering|Material|SetMaterial _rootmesh 0 "/Game/Material/M_DisallowToSpawn.M_DisallowToSpawn")
      (Rendering|Material|SetMaterial _rootmesh 1 "/Game/Material/M_DisallowToSpawn.M_DisallowToSpawn"))))