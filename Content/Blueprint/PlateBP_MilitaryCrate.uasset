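; PlateBP_MilitaryCrate is a placeable military crate that shows whether it can be spawned at its preview position.
; It extends a parent placement Blueprint, calling the parent logic in both of its overrides.
; Select Preview Mesh swaps the root mesh's first material between allow and disallow materials based on CanSpawn.
; Set Real Actor restores the original material on that slot when the crate becomes the real actor.
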(fn ConstructionScript)

(fn SetRealActor
  (|CallParentFunction)
  (Rendering|Material|SetMaterial (Variables|Default|GetRootMesh) 0 (Variables|Default|GetoriginMaterial%201)))

(fn SelectPreviewMesh
  (params (bPlacable :type Boolean))
  (bind _rootmesh (Variables|Default|GetRootMesh))
  (|CallParentFunction bPlacable)
  (if (Variables|Default|GetbCanSpawn)
    (Rendering|Material|SetMaterial _rootmesh 0 "/Game/Material/M_AllowToSpawn.M_AllowToSpawn")
    (else
      (Rendering|Material|SetMaterial _rootmesh 0 "/Game/Material/M_DisallowToSpawn.M_DisallowToSpawn"))))