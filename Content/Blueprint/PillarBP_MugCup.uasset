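; Mug cup pillar Blueprint, a placeable actor that shows whether it can spawn while in preview.
; It extends two parent functions to handle the two material slots on its root mesh.
; Select Preview Mesh calls the parent, then applies an allow or disallow material to both slots based on CanSpawn.
; Set Real Actor calls the parent, then applies the original material to each slot.
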(event Collision|EventActorBeginOverlap
  (params (OtherActor :type Actor%20Object%20Reference)))

(event EventTick
  (params (DeltaSeconds :type Float%20%28single-precision%29)))

(fn ConstructionScript)

(fn SetRealActor
  (bind _rootmesh (Variables|Default|GetRootMesh))
  (|CallParentFunction)
  (Rendering|Material|SetMaterial _rootmesh 0 (Variables|Default|GetoriginMaterial%201))
  (Rendering|Material|SetMaterial _rootmesh 1 (Variables|Default|GetoriginMaterial%202)))

(fn SelectPreviewMesh
  (params (bPlacable :type Boolean))
  (bind _rootmesh (Variables|Default|GetRootMesh))
  (|CallParentFunction bPlacable)
  (if (Variables|Default|GetbCanSpawn)
    (Rendering|Material|SetMaterial _rootmesh 0 "/Game/Material/M_AllowToSpawn.M_AllowToSpawn")
    (Rendering|Material|SetMaterial _rootmesh 1 "/Game/Material/M_AllowToSpawn.M_AllowToSpawn")
    (else
      (Rendering|Material|SetMaterial _rootmesh 0 "/Game/Material/M_DisallowToSpawn.M_DisallowToSpawn")
      (Rendering|Material|SetMaterial _rootmesh 1 "/Game/Material/M_DisallowToSpawn.M_DisallowToSpawn"))))