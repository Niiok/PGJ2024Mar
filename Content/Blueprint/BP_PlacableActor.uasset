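; Placeable actor that tracks whether it is a preview or a real, spawned actor through an IsSpawned flag.
; BeginPlay switches it to real, and SetPreviewActor and SetRealActor only flip the flag, with no visual or collision changes.
; An OnRep-named handler calls the setter matching the flag's current value, so their guards make that call a no-op.
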(event EventBeginPlay
  (CallFunction|SetRealActor))

(event Collision|EventActorBeginOverlap
  (params (OtherActor :type Actor%20Object%20Reference)))

(event EventTick
  (params (DeltaSeconds :type Float%20%28single-precision%29)))

(fn ConstructionScript)

(fn SetPreviewActor
  (if (Variables|Default|GetbIsSpawned)
    (Variables|Default|SetbIsSpawned false)))

(fn SetRealActor
  (if (not (Variables|Default|GetbIsSpawned))
    (Variables|Default|SetbIsSpawned true)))

(fn OnRepBIsSpawned
  (if (Variables|Default|GetbIsSpawned)
    (CallFunction|SetRealActor)
    (else
      (CallFunction|SetPreviewActor))))