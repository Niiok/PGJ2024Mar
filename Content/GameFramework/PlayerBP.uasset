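; Player pawn that places objects in the level and controls a spring-arm camera.
; Holding left mouse spawns a preview of SelectedClass, which a gated, locally controlled Tick snaps to the cursor hit and surface normal.
; Release destroys the preview; if CanSpawn, PGPlayerController first spawns the real actor, then the InGameLevelGM timer resets and a sound plays.
; Right-drag rotates the view, Q/E move vertically, and the wheel zooms.
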(event EventBeginPlay
  (bind _springarm (Variables|Default|GetSpringArm))
  ;[1 1 1] 초기화
  (Variables|Default|SetSelected%20Class 0)
  (Transformation|SetWorldLocationAndRotation _springarm "0, 0, 0" "0, 0, 0" false false)
  (bind _asplayer_controller (Utilities|Casting|CastToPlayerController (Pawn|GetController)))
  (Pawn|SetControlRotation _asplayer_controller (Math|Rotator|MakeRotator 0.0 -2e+01 2.3e+02))
  (Variables|/Script/Engine.SpringArmComponent|SetTargetArmLength _springarm 6e+02))

(event Collision|EventActorBeginOverlap
  (params (OtherActor :type Actor%20Object%20Reference)))

(event EventTick
  (params (DeltaSeconds :type Float%20%28single-precision%29))
  (if (Pawn|IsLocallyControlled)
    (Utilities|FlowControl|Sequence
      (:then_0
        ;[1 1 1] 오브젝트 생성
        (Utilities|FlowControl|Gate true
          (:Exit
            (bind _asplayer_controller (Utilities|Casting|CastToPlayerController (Pawn|GetController)))
            (Transformation|SetActorLocationAndRotation (Variables|Default|GetPreview%20Actor) (+ (.Location (Collision|BreakHitResult (.HitResult (Class|PlayerController|GetHitResultUnderCursorforObjects _asplayer_controller (Utilities|Array|MakeArray "ObjectTypeQuery8") true)))) (.Normal (Collision|BreakHitResult (.HitResult (Class|PlayerController|GetHitResultUnderCursorforObjects _asplayer_controller (Utilities|Array|MakeArray "ObjectTypeQuery8") true))))) (Math|Rotator|MakeRotfromZ (.Normal (Collision|BreakHitResult (.HitResult (Class|PlayerController|GetHitResultUnderCursorforObjects _asplayer_controller (Utilities|Array|MakeArray "ObjectTypeQuery8") true)))))))))
      (:then_1
        ;[1 1 1] 카메라 움직임
        (Utilities|FlowControl|Sequence
          (:then_0
            (if (Variables|Default|GetCameraUp)
              (Pawn|Input|AddMovementInput "0, 0,1.000000" 1.0 false)))
          (:then_1
            (if (Variables|Default|GetCameraDown)
              (Pawn|Input|AddMovementInput "0, 0,1.000000" -1.0 false))))))))

(event Input|MouseEvents|MouseX
  (params (AxisValue :type Float%20%28single-precision%29))
  ;[1 1 1] 카메라 움직임
  (if (Variables|Default|GetCameraMovable)
    (Pawn|Input|AddControllerYawInput AxisValue)))

(event Input|MouseEvents|MouseY
  (params (AxisValue :type Float%20%28single-precision%29))
  ;[1 1 1] 카메라 움직임
  (if (Variables|Default|GetCameraMovable)
    (Pawn|Input|AddControllerPitchInput (* AxisValue -1.0))))

(event Input|MouseEvents|MouseWheelAxis
  (params (AxisValue :type Float%20%28single-precision%29))
  (bind _springarm (Variables|Default|GetSpringArm))
  ;[1 1 1] 카메라 움직임
  (Variables|/Script/Engine.SpringArmComponent|SetTargetArmLength _springarm (- (Variables|/Script/Engine.SpringArmComponent|GetTargetArmLength _springarm) (* AxisValue 2e+01))))

(event Input|MouseEvents|LeftMouseButton
  (params (Key :type Key%20Structure :default "None"))
  ;[1 1 1] 오브젝트 생성
  (:Pressed
    (if (Utilities|IsValidClass (Variables|Default|GetSelected%20Class))
      (CallFunction|SpawnPreviewActor)
      (Utilities|FlowControl|Gate true) ; enters at Open
    ))
  (:Released
    (if (Utilities|IsValid (Variables|Default|GetPreview%20Actor))
      (Utilities|FlowControl|Sequence
        (:then_0
          (bind _can_spawn (CallFunction|CheckObjectCanSpawn))
          (if _can_spawn
            (CallFunction|SpawnRealActor)))
        (:then_1
          (Actor|DestroyActor (Variables|Default|GetPreview%20Actor))
          (Utilities|FlowControl|Gate true) ; enters at Close
        )))))

(event Input|MouseEvents|RightMouseButton
  (params (Key :type Key%20Structure :default "None"))
  ;[1 1 1] 카메라 움직임
  (:Pressed
    (Variables|Default|SetCameraMovable true))
  (:Released
    (Variables|Default|SetCameraMovable false)))

(event Input|KeyboardEvents|Q
  (params (Key :type Key%20Structure :default "None"))
  ;[1 1 1] 카메라 움직임
  (:Pressed
    (Variables|Default|SetCameraUp true))
  (:Released
    (Variables|Default|SetCameraUp false)))

(event Input|KeyboardEvents|E
  (params (Key :type Key%20Structure :default "None"))
  ;[1 1 1] 카메라 움직임
  (:Pressed
    (Variables|Default|SetCameraDown true))
  (:Released
    (Variables|Default|SetCameraDown false)))

(fn ConstructionScript)

(fn SpawnPreviewActor
  (bind _returnvalue (Game|SpawnActorfromClass (Variables|Default|GetSelected%20Class) (Transformation|GetActorTransform) "Undefined" 0 0))
  (bind _asbp_placable_actor (Utilities|Casting|CastToBP_PlacableActor _returnvalue))
  (bind _output_get (Variables|Default|SetPreview%20Actor _asbp_placable_actor))
  (Default|SetPreviewActor _output_get))

(fn CheckObjectCanSpawn
  (return (Variables|/Game/Blueprint/BP_PlacableActor.BP_PlacableActor_C|GetbCanSpawn (Variables|Default|GetPreview%20Actor))))

(fn SpawnRealActor
  (bind _aspgplayer_controller (Utilities|Casting|CastToPGPlayerController (Pawn|GetController)))
  (bind _returnvalue (Class|PGPlayerController|SpawnActorBlueprint _aspgplayer_controller (Variables|Default|GetSelected%20Class) (Transformation|GetActorTransform (Variables|Default|GetPreview%20Actor))))
  (bind _asbp_placable_actor (Utilities|Casting|CastToBP_PlacableActor _returnvalue))
  (Default|SetRealActor _asbp_placable_actor)
  (bind _asin_game_level_gm (Utilities|Casting|CastToInGameLevelGM (Game|GetGameMode)))
  (Default|ResetTimer _asin_game_level_gm)
  (Audio|PlaySound2D "/Game/Sounds/multi-pop-1-188165.multi-pop-1-188165" 1.0 1.0 0.0 0 0))