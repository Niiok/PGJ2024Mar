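; Game instance that runs online multiplayer matchmaking for PillarGame through the EOS subsystem.
; StartMulti logs in with device-ID credentials if needed, then searches for a keyword-tagged session and joins the first result.
; If none is found or the search fails, it creates an advertised session and opens ControlTestRoom as a listen server.
; A busy flag blocks overlapping attempts, and Shutdown logs the player out.
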(event Custom|Start%20Multi
  (bind _returnvalue (Class|GameplayStatics|GetPlayerControllerfromID))
  (bind _returnvalue_2 (Subsystems|GetEOSSubsystem))
  (if (not (Variables|Default|GetbIsBusy))
    (Variables|Default|SetbIsBusy true)
    (if (Variables|Default|GetbLoggedIn)
      (bind _results (|FindSessionswithParam _returnvalue 1 false (Class|EOSSubsystem|SetSearchSessionKeyword _returnvalue_2 (Utilities|Struct|MakeOnlineSearchSettings) "PillarGame") :!label _label)
        (:OnSuccess
          (if (> (Utilities|Array|Length _results) 0)
            (|JoinSession _returnvalue (Utilities|Array|Get(acopy) _results)
              (:OnSuccess
                _)
              (:OnFailure
                _))
            (else
              (|SessionwithSetting _returnvalue (Class|EOSSubsystem|SetCreateSessionKeyword _returnvalue_2 (Utilities|Struct|MakeOnlineSessionSettings 3 0 true true false false false false true true) "PillarGame") :!label _label_2
                (:OnSuccess
                  (Game|OpenLevel(byObjectReference) "/Game/Level/ControlTestRoom.ControlTestRoom" true "listen"))
                (:OnFailure
                  _)))))
        (:OnFailure
          (goto _label_2)))
      (Variables|Default|SetbIsBusy false)
      (else
        (|LoginwithCredentials _returnvalue (Utilities|Struct|MakeOnlineAccountCredentials "deviceid")
          (:OnSuccess
            (Variables|Default|SetbLoggedIn true)
            (goto _label))
          (:OnFailure
            (Variables|Default|SetbIsBusy false)))))))

(event EventShutdown
  (|Logout (Class|GameplayStatics|GetPlayerControllerfromID)))

(fn IsBusy
  (return (Variables|Default|GetbIsBusy)))